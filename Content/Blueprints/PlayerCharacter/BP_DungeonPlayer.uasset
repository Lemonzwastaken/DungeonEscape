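; First-person dungeon player character that adds procedural head bob and idle breathing sway to its camera.
; Each tick, a grounded-only timer drives sine-wave camera height and roll, with frequency and amplitude scaled by speed between walk and sprint settings.
; A separate idle timer adds breathing pitch that fades out as speed rises.
; Interpolation smooths both offsets, and both tick events share the rotation update, so it runs twice per frame.
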(event `self.ReceiveBeginPlay`
  (`|ExecutionSequence`
    (:`then_0`
      (set `self.DefaultCameraLoc` (`SceneComponent.RelativeLocation` (`self.FirstPersonCameraComponent`))))))

(event `self.ReceiveTick`
  (params (DeltaSeconds :type "Float (single-precision)"))
  (`|ExecutionSequence`
    (:`then_0`
      (`self.HeadBobbing`))
    (:`then_1`
      (`self.IdleBob`))))

(event `HeadBobbing`
  (bind _returnvalue (`GameplayStatics.GetWorldDeltaSeconds`))
  (bind _firstpersoncameracomponent (`self.FirstPersonCameraComponent`))
  (bind _returnvalue_2 (`KismetMathLibrary.VSize` (`self.GetVelocity`)))
  (bind _returnvalue_3 (`MovementComponent.GetMaxSpeed` (`self.CharacterMovement`)))
  (bind _returnvalue_4 (`KismetMathLibrary.MapRangeClamped` _returnvalue_2 0.0 _returnvalue_3 0.0 1.0))
  (bind _returnvalue_5 (* (`KismetMathLibrary.Lerp` (`self.WalkBoBHeightRoll`) (`self.SprintBobHeightRoll`) _returnvalue_4) _returnvalue_4))
  ; HeadBobbing
  (if (and (`self.CanJump`) (`NavMovementComponent.IsMovingOnGround` (`self.CharacterMovement`)))
    (set `self.HeadBobTimer` (+ (`self.HeadBobTimer`) (* (`GameplayStatics.GetWorldDeltaSeconds`) (`KismetMathLibrary.Lerp` (`self.WalkFrequency`) (`self.SprintFrequency`) (`KismetMathLibrary.MapRangeClamped` _returnvalue_2 0.0 _returnvalue_3 0.0 1.0)))))
    (else
      (set `self.HeadBobTimer` 0.0)))
  (`SceneComponent.K2_SetRelativeLocation` _firstpersoncameracomponent (`KismetMathLibrary.VInterpTo` (`SceneComponent.RelativeLocation` (`self.FirstPersonCameraComponent`)) (+ (`KismetMathLibrary.MakeVector` 0.0 0.0 (* (* (`KismetMathLibrary.Sin` (`self.HeadBobTimer`)) _returnvalue_5) (`self.BobHeight`))) (`self.DefaultCameraLoc`)) _returnvalue (`self.InterpSpeed`)) false false)
  (`SceneComponent.K2_SetRelativeRotation` _firstpersoncameracomponent (`KismetMathLibrary.RInterpTo` (`SceneComponent.RelativeRotation` (`self.FirstPersonCameraComponent`)) (`KismetMathLibrary.MakeRotator` (* (* _returnvalue_5 (`KismetMathLibrary.Sin` (* (`self.HeadBobTimer`) 0.5))) (`self.BobRoll`)) (* (* (`KismetMathLibrary.Sin` (* (`self.IdleTimer`) 2.0)) (`self.IdlePitch`)) (`KismetMathLibrary.MapRangeClamped` _returnvalue_2 0.0 300.0 1.0))) _returnvalue (`self.InterpSpeed`)) false false :!label _label))

(event `IdleBob`
  ; HeadBobbing
  (set `self.IdleTimer` (+ (`GameplayStatics.GetWorldDeltaSeconds`) (`self.IdleTimer`)))
  (goto _label))

(fn `UserConstructionScript`
  (`parent.UserConstructionScript`))